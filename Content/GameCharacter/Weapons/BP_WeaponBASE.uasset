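; BP_WeaponBASE is the base Blueprint for weapons, providing equip, unequip and fire functions.
; Equip and Unequip show or hide the actor and toggle its collision to match.
; Fire checks that an AnimMontage is set, casts the stored Character to BP_Player and plays the montage on it.
; It contains no damage or projectile logic, and its event graph is empty apart from disabled default events.
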(event EventBeginPlay)

(event Collision|EventActorBeginOverlap
  (params (OtherActor :type Actor%20Object%20Reference)))

(event EventTick
  (params (DeltaSeconds :type Float%20%28single-precision%29)))

(fn ConstructionScript)

(fn Equip
  (Rendering|SetActorHiddenInGame false)
  (Collision|SetActorEnableCollision true))

(fn Unequip
  (Rendering|SetActorHiddenInGame true)
  (Collision|SetActorEnableCollision false))

(fn Fire
  (bind _animmontage (Variables|Default|GetAnimMontage))
  (Utilities|IsValid _animmontage
    (:Is%20Valid
      (bind _asbp_player (Utilities|Casting|CastToBP_Player (Variables|Default|GetCharacter)))
      (Animation|PlayAnimMontage _asbp_player _animmontage 1.0 "None"))))