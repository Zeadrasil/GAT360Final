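; Player character Blueprint that carries a set of weapons, cycles through them and fires the current one through Enhanced Input actions.
; BeginPlay spawns each SpawnWeapons class onto its mesh socket, unequips all, equips the first and sets jump velocity.
; EquipWeapon swaps the current weapon and sets walk speed by weapon type, with swords slower than no weapon type.
; Tick steadily raises the Niagara ashfall rate with elapsed time.
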(event Custom|Set%20Speed
  (bind _charactermovement (Variables|Character|GetCharacterMovement))
  ;[1 1 1] Set Speed Based On Equipped Weapon
  (switch Utilities|FlowControl|Switch|SwitchonEWeaponType (Variables|/Game/GameCharacter/Weapons/BP_WeaponBASE.BP_WeaponBASE_C|GetWeaponType (Variables|Default|GetCurrentWeapon))
    (:NewEnumerator0
      (Variables|/Script/Engine.CharacterMovementComponent|SetMaxWalkSpeed _charactermovement 5e+02))
    (:NewEnumerator1
      (Variables|/Script/Engine.CharacterMovementComponent|SetMaxWalkSpeed _charactermovement 3e+02))))

(event Input|EnhancedActionEvents|EnhancedInputActionIA_SwitchWeapon
  (params (ActionValue :type Boolean) (ElapsedSeconds :type Float%20%28double-precision%29) (TriggeredSeconds :type Float%20%28double-precision%29) (InputAction :type Input%20Action%20Object%20Reference :default "/Game/GameCharacter/InputActions/IA_SwitchWeapon.IA_SwitchWeapon"))
  (bind _weapons (Variables|Default|GetWeapons))
  ;[1 1 1] Switch Weapon
  (bind _result (Math|Integer|IncrementInt (Utilities|Array|FindItem _weapons (Variables|Default|GetCurrentWeapon)))
    (:%20%20
      (CallFunction|EquipWeapon (Utilities|Array|Get(acopy) _weapons (Math|Integer|%(Integer) _result (Utilities|Array|Length _weapons)))))))

(event Input|EnhancedActionEvents|EnhancedInputActionIA_UseWeapon
  (params (ActionValue :type Boolean) (ElapsedSeconds :type Float%20%28double-precision%29) (TriggeredSeconds :type Float%20%28double-precision%29) (InputAction :type Input%20Action%20Object%20Reference :default "/Game/GameCharacter/InputActions/IA_UseWeapon.IA_UseWeapon"))
  ;[1 1 1] Use Weapon
  (Default|Fire (Variables|Default|GetCurrentWeapon)))

(event EventBeginPlay
  (Utilities|FlowControl|Sequence
    (:then_0
      ;[1 1 1] Add All Spawn Weapons
      (for _array_element (Variables|Default|GetSpawnWeapons)
        (bind _returnvalue (Game|SpawnActorfromClass _array_element (Transformation|GetActorTransform) "Undefined" "MultiplyWithRoot" 0 self 0))
        (Transformation|AttachComponentToComponent _returnvalue (Variables|Character|GetMesh) (Variables|/Game/GameCharacter/Weapons/BP_WeaponBASE.BP_WeaponBASE_C|GetSocketName _returnvalue) "SnapToTarget" "SnapToTarget" "KeepRelative" true)
        (Utilities|Array|Add (Variables|Default|GetWeapons) _returnvalue)))
    (:then_1
      ;[1 1 1] Unequip all weapons
      (for _array_element_2 (Variables|Default|GetWeapons)
        (Default|Unequip _array_element_2)))
    (:then_2
      ;[1 1 1] EquipWeapon
      (CallFunction|EquipWeapon (Utilities|Array|Get(acopy) (Variables|Default|GetWeapons))))
    (:then_3
      (Variables|/Script/Engine.CharacterMovementComponent|SetJumpZVelocity (Variables|Character|GetCharacterMovement) 1.15e+03))))

(event Collision|EventActorBeginOverlap
  (params (OtherActor :type Actor%20Object%20Reference)))

(event EventTick
  (params (DeltaSeconds :type Float%20%28single-precision%29))
  (Effects|Components|ParticleSystem|SetFloatParameter (Variables|Default|GetNiagara) "ashfallRate" (* (Actor|GetGameTimeSinceCreation) 2.0)))

(fn ConstructionScript)

(fn EquipWeapon
  (params (NewWeapon :type BP%20Weapon%20BASE%20Object%20Reference))
  (Utilities|IsValid (Variables|Default|GetCurrentWeapon)
    (:Is%20Valid
      (Default|Unequip (Variables|Default|GetCurrentWeapon)))
    (:Is%20Not%20Valid
      _))
  (bind _output_get (Variables|Default|SetCurrentWeapon NewWeapon))
  (Default|Equip _output_get)
  (CallFunction|SetSpeed))