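; BP_Lava is a lava hazard actor that rises continuously and detects contact with the player.
; Tick moves the Cube component up along its relative Z axis at MovementSpeed, scaled by delta time for frame-rate independence.
; Actor overlap with player character 0 only prints "Dead", with no damage or death logic.
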(event EventBeginPlay)

(event EventTick
  (params (DeltaSeconds :type Float%20%28single-precision%29))
  (bind _cube (Variables|Default|GetCube))
  (bind _returnvalue (Transformation|GetRelativeTransform _cube))
  (Transformation|SetRelativeLocation _cube (Math|Vector|MakeVector (.x (.location _returnvalue)) (.y (.location _returnvalue)) (+ (.z (.location _returnvalue)) (* DeltaSeconds (Variables|Default|GetmovementSpeed)))) false false))

(event Collision|EventActorBeginOverlap
  (params (OtherActor :type Actor%20Object%20Reference))
  (if (== OtherActor (Game|GetPlayerCharacter 0))
    (Development|PrintString "Dead")))

(fn ConstructionScript)